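; Game mode that handles player join, pawn spawning and swapping, and test enemy spawning.
; On authority, each login is tracked, PlayerStarts are gathered, the player is respawned at a random one and the controller sets up its lobby menu.
; Respawn and character swap destroy the current pawn, then spawn and possess a new one.
; SpawnEnemies runs an EQS query and spawns a BP_TestEnemy at the returned location.
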(event `self.K2_PostLogin`
  (params (NewPlayer :type "PlayerController Object Reference"))
  (`/Engine/EditorBlueprintResources/ActorMacros.Switch Has Authority`
    (:`Authority`
      (`KismetArrayLibrary.Array_Add` (`self.AllPlayerControllers`) NewPlayer)
      (bind _outactors (`GameplayStatics.GetAllActorsOfClass` "/Script/Engine.PlayerStart"))
      (set `self.SpawnPoints` _outactors)
      (`self.RespawnPlayer` NewPlayer)
      (bind _asbp_player_controller (cast `/Game/Blueprints/BP_PlayerController` NewPlayer))
      (`/Game/Blueprints/BP_PlayerController.SetupLobbyMenu` _asbp_player_controller))))

(event `RespawnPlayer`
  (params (PlayerController :type "PlayerController Object Reference"))
  (bind _returnvalue (`Controller.K2_GetPawn` PlayerController))
  (bind _spawnpoints (`self.SpawnPoints`))
  (`/Engine/EditorBlueprintResources/StandardMacros.IsValid` _returnvalue
    (:`Is Valid`
      (`self.K2_DestroyActor` _returnvalue))
    (:`Is Not Valid`
      _))
  (bind _returnvalue_2 (`|SpawnActorFromClass` "/Script/Engine.Character" (`self.GetTransform` (`|GetArrayItem` _spawnpoints (`KismetMathLibrary.RandomIntegerInRange` 0 (- (`KismetArrayLibrary.Array_Length` _spawnpoints) 1)))) "Undefined" "OverrideRootScale" null null))
  (`Controller.Possess` PlayerController _returnvalue_2))

(event `self.SpawnEnemies`
  (bind _returnvalue (`EnvQueryManager.RunEQSQuery` "/Game/Blueprints/EQS/EQS_SpawnLocation.EQS_SpawnLocation" self "RandomBest25Pct"))
  (add `EnvQueryInstanceBlueprintWrapper.OnQueryFinishedEvent` _returnvalue (delegate `OnQueryFinishedEvent_Event_0`)))

(event `SwapCharacter`
  (params (PlayerController :type "PlayerController Object Reference") (CharacterClass :type "Character Class Reference"))
  (bind _returnvalue (`Controller.K2_GetPawn` PlayerController))
  (bind _spawnpoints (`self.SpawnPoints`))
  (if (`KismetSystemLibrary.IsValidClass` CharacterClass)
    (`/Engine/EditorBlueprintResources/StandardMacros.IsValid` _returnvalue
      (:`Is Valid`
        (`self.K2_DestroyActor` _returnvalue))
      (:`Is Not Valid`
        _))
    (bind _returnvalue_2 (`|SpawnActorFromClass` CharacterClass (`self.GetTransform` (`|GetArrayItem` _spawnpoints (`KismetMathLibrary.RandomIntegerInRange` 0 (- (`KismetArrayLibrary.Array_Length` _spawnpoints) 1)))) "Undefined" "OverrideRootScale" null null))
    (`Controller.Possess` PlayerController _returnvalue_2)
    (else
      (`KismetSystemLibrary.PrintString` "Could not find a valid class"))))

(event `OnQueryFinishedEvent_Event_0`
  (params (QueryInstance :type "EnvQueryInstanceBlueprintWrapper Object Reference") (QueryStatus :type "EEnvQueryStatus Enum" :default "Processing"))
  (switch `EEnvQueryStatus` QueryStatus
    (:`Success`
      (bind _resultlocations (`EnvQueryInstanceBlueprintWrapper.GetQueryResultsAsLocations` QueryInstance))
      (`AIBlueprintHelperLibrary.SpawnAIFromClass` "/Game/Blueprints/Character/BP_TestEnemy.BP_TestEnemy_C" null (`|GetArrayItem` _resultlocations) (struct) true null))))

(fn `UserConstructionScript`)