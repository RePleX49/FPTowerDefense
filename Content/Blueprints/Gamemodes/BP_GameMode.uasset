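; Multiplayer game mode that handles player joins, random-point spawning and character swapping.
; On authority, PostLogin records each controller, caches all PlayerStarts, spawns a pawn through RespawnPlayer and opens the lobby menu on BP_PlayerController.
; RespawnPlayer and SwapCharacter destroy the current pawn, then possess a new one at a random start, using the default or supplied class respectively.
; GetDefaultPawnClassForController prefers the controller's PlayerClass, falling back to the parent implementation.
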(event `self.K2_PostLogin`
  (params (NewPlayer :type "PlayerController Object Reference"))
  (`/Engine/EditorBlueprintResources/ActorMacros.Switch Has Authority`
    (:`Authority`
      (`KismetArrayLibrary.Array_Add` (`self.AllPlayerControllers`) NewPlayer)
      (bind _outactors (`GameplayStatics.GetAllActorsOfClass` "/Script/Engine.PlayerStart"))
      (set `self.SpawnPoints` _outactors)
      (`self.RespawnPlayer` NewPlayer)
      (bind _asbp_player_controller (cast `/Game/Blueprints/BP_PlayerController` NewPlayer))
      (`/Game/Blueprints/BP_PlayerController.SetupLobbyMenu` _asbp_player_controller))))

(event `RespawnPlayer`
  (params (PlayerController :type "PlayerController Object Reference"))
  (bind _returnvalue (`Controller.K2_GetPawn` PlayerController))
  (bind _spawnpoints (`self.SpawnPoints`))
  (`/Engine/EditorBlueprintResources/StandardMacros.IsValid` _returnvalue
    (:`Is Valid`
      (`self.K2_DestroyActor` _returnvalue))
    (:`Is Not Valid`
      _))
  (bind _returnvalue_2 (`|SpawnActorFromClass` "/Script/Engine.Character" (`self.GetTransform` (`|GetArrayItem` _spawnpoints (`KismetMathLibrary.RandomIntegerInRange` 0 (- (`KismetArrayLibrary.Array_Length` _spawnpoints) 1)))) "Undefined" "OverrideRootScale" null null))
  (`Controller.Possess` PlayerController _returnvalue_2))

(event `SwapCharacter`
  (params (PlayerController :type "PlayerController Object Reference") (CharacterClass :type "Character Class Reference"))
  (bind _returnvalue (`Controller.K2_GetPawn` PlayerController))
  (bind _spawnpoints (`self.SpawnPoints`))
  (if (`KismetSystemLibrary.IsValidClass` CharacterClass)
    (`/Engine/EditorBlueprintResources/StandardMacros.IsValid` _returnvalue
      (:`Is Valid`
        (`self.K2_DestroyActor` _returnvalue))
      (:`Is Not Valid`
        _))
    (bind _returnvalue_2 (`|SpawnActorFromClass` CharacterClass (`self.GetTransform` (`|GetArrayItem` _spawnpoints (`KismetMathLibrary.RandomIntegerInRange` 0 (- (`KismetArrayLibrary.Array_Length` _spawnpoints) 1)))) "Undefined" "OverrideRootScale" null null))
    (`Controller.Possess` PlayerController _returnvalue_2)
    (else
      (`KismetSystemLibrary.PrintString` "Could not find a valid class"))))

(fn `GetDefaultPawnClassForController`
  (params (InController :type "Controller Object Reference"))
  (returns (ReturnValue :type "Object Class Reference"))
  (bind _asbp_player_controller (cast `/Game/Blueprints/BP_PlayerController` InController)
    (:`then`
      (bind _playerclass (`/Game/Blueprints/BP_PlayerController.PlayerClass` _asbp_player_controller))
      (if (`KismetSystemLibrary.IsValidClass` _playerclass)
        (return _playerclass)
        (else
          _)))
    (:`CastFailed`
      _))
  (bind _returnvalue (`parent.GetDefaultPawnClassForController` null))
  (return _returnvalue))

(fn `UserConstructionScript`)