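; Black hole ability actor that drags enemies toward its center.
; Each Tick it finds FEnemy actors overlapping Sphere1 and, unless they are closer than MinDistance, pushes their CharacterMovement toward itself with a DrawForce-scaled force that does not vary with distance.
; A radial-force variant for physics-simulating components is left in the graph but never runs.
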(event `self.ReceiveTick`
  (params (DeltaSeconds :type "Float (single-precision)"))
  (for _array_element (`PrimitiveComponent.GetOverlappingActors` (`self.Sphere1`) "/Script/FPTowerDefense.FEnemy")
    (if (not (< (`self.GetDistanceTo` _array_element self) (`self.MinDistance`)))
      (bind _asfenemy (cast `FEnemy` _array_element))
      (`CharacterMovementComponent.AddForce` (`Character.CharacterMovement` _asfenemy) (* (`KismetMathLibrary.Normal` (- (`self.K2_GetActorLocation`) (`self.K2_GetActorLocation` _array_element))) (`self.DrawForce`))))))

(fn `UserConstructionScript`)