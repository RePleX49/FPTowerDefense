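; Player character Blueprint that creates the weapon UI on begin play and plays RU74 reload and fire montages on its arm mesh.
; Fire animation starts only if its timer is inactive, then repeats at an interval derived from the equipped weapon's fire rate.
; Each loop replays the montage and sets the timer again, until EndFireAnim clears the handle.
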(event `self.ReceiveBeginPlay`
  (bind _returnvalue (`|CreateWidget` "/Game/Blueprints/Widgets/WBP_WeaponUI.WBP_WeaponUI_C" (`GameplayStatics.GetPlayerController` 0)))
  (`UserWidget.AddToViewport` _returnvalue 0))

(event `self.PlayReloadAnim`
  (`|PlayMontage` (`self.ArmMesh`) "/Game/FPS_Assault_Pack/Animations/RU74/A_Arms_RU74_Reload_Empty_Montage.A_Arms_RU74_Reload_Empty_Montage"))

(event `self.PlayFireAnim`
  (if (not (`KismetSystemLibrary.K2_IsTimerActiveHandle` (`self.TimerHandle_Fire`)))
    (`|PlayMontage` (`self.ArmMesh`) "/Game/FPS_Assault_Pack/Animations/RU74/A_Arms_RU74_Shoot01_Montage.A_Arms_RU74_Shoot01_Montage" :!label _label
      (:`then`
        (bind _returnvalue (`KismetSystemLibrary.K2_SetTimerDelegate` (delegate `LoopFireAnim`) (/ 60.0 (`FWeapon.FireRate` (`self.EquippedWeapon`))) true 0.0 0.02))
        (set `self.TimerHandle_Fire` _returnvalue)))))

(event `LoopFireAnim`
  (goto _label))

(event `self.EndFireAnim`
  (`KismetSystemLibrary.K2_ClearAndInvalidateTimerHandle` (`self.TimerHandle_Fire`)))

(fn `UserConstructionScript`)