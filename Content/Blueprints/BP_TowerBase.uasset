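; BP_TowerBase is a tower base actor that turns its UI pivot to face a nearby character.
; Overlap events detect an FCharacter, store it as the user on entry, and toggle an in-range flag on entry and exit.
; While the flag is set, Tick sets the pivot's world rotation to a full look-at rotation toward that character's location.
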(event `self.ReceiveActorBeginOverlap`
  (params (OtherActor :type "Actor Object Reference"))
  (bind _asfcharacter (cast `FCharacter` OtherActor))
  (set `self.UserCharacter` _asfcharacter)
  (set `self.bUserInRange` true))

(event `self.ReceiveActorEndOverlap`
  (params (OtherActor :type "Actor Object Reference"))
  (cast `FCharacter` OtherActor)
  (set `self.bUserInRange` false))

(event `self.ReceiveTick`
  (params (DeltaSeconds :type "Float (single-precision)"))
  (bind _ui_pivot (`self.UI_Pivot`))
  (if (`self.bUserInRange`)
    (`SceneComponent.K2_SetWorldRotation` _ui_pivot (`KismetMathLibrary.MakeRotator` (.roll (`KismetMathLibrary.FindLookAtRotation` (`SceneComponent.K2_GetComponentLocation` _ui_pivot) (`self.K2_GetActorLocation` (`self.UserCharacter`)))) (.pitch (`KismetMathLibrary.FindLookAtRotation` (`SceneComponent.K2_GetComponentLocation` _ui_pivot) (`self.K2_GetActorLocation` (`self.UserCharacter`)))) (.yaw (`KismetMathLibrary.FindLookAtRotation` (`SceneComponent.K2_GetComponentLocation` _ui_pivot) (`self.K2_GetActorLocation` (`self.UserCharacter`))))) false false)))

(fn `UserConstructionScript`)