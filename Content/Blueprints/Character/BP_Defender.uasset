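; BP_Defender is the Defender character Blueprint, implementing its two abilities and creating its weapon HUD.
; The offensive ability uses a temporary sphere collider to restore a quarter of max shield to overlapping characters, with a debug sphere showing the radius.
; The support ability spawns a BP_Shield at a scene component's transform.
; Camera-trace targeting for a single-target shield repair remains but never runs, and GetDistance is unfinished.
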(event `Key|C`
  (params (Key :type "Key Structure")))

(event `self.UseOffensiveBP`
  (bind _buffspherecollider (`self.BuffSphereCollider`))
  (bind _returnvalue (`AddComponent|NODE_AddSphereComponent-0`))
  (set `self.BuffSphereCollider` _returnvalue)
  (`PrimitiveComponent.SetCollisionResponseToChannel` _buffspherecollider "ECC_GameTraceChannel1" "ECR_Overlap")
  (`SphereComponent.SetSphereRadius` _buffspherecollider 1000.0 true)
  (`KismetSystemLibrary.DrawDebugSphere` (`self.K2_GetActorLocation`) 1000.0 12 (struct :`R` 1.0 :`G` 1.0 :`B` 1.0 :`A` 1.0) 2.0 1.0)
  (for _array_element (`PrimitiveComponent.GetOverlappingActors` _buffspherecollider "/Script/FPTowerDefense.FCharacter")
    (bind _asfcharacter (cast `FCharacter` _array_element))
    (bind _healthcomp (`FCharacter.HealthComp` _asfcharacter))
    (`FHealthComponent.RepairShield` _healthcomp (* (`FHealthComponent.MaxShield` _healthcomp) 0.25)))
  (`ActorComponent.K2_DestroyComponent` (`self.BuffSphereCollider`)))

(event `self.UseSupportBP`
  (`|SpawnActorFromClass` "/Game/Blueprints/Abilities/BP_Shield.BP_Shield_C" (`SceneComponent.K2_GetComponentToWorld` (`self.Scene`)) "AlwaysSpawn" "OverrideRootScale" null null))

(event `SetupUI`
  (bind _returnvalue (`GameplayStatics.GetPlayerController` 0))
  (`WidgetLayoutLibrary.RemoveAllWidgets`)
  (bind _returnvalue_2 (`|CreateWidget` "/Game/Blueprints/Widgets/WBP_WeaponUI.WBP_WeaponUI_C" _returnvalue))
  (bind _output_get (set `self.WBP_Weapon` _returnvalue_2))
  (`UserWidget.AddToViewport` _output_get 0)
  (set `PlayerController.bShowMouseCursor` false _returnvalue)
  (`WidgetBlueprintLibrary.SetInputMode_GameOnly` _returnvalue))

(fn `UserConstructionScript`)