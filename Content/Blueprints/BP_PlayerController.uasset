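; Player controller that handles the lobby menu, character selection, ready state and in-game UI setup.
; It creates the lobby widget with UI-only input, then maps the selected character ID to a game mode class and requests a pawn swap.
; Ready and unready toggles are guarded and reported to BP_FTDGameMode.
; Possessing a Defender or Trapper triggers that pawn's UI setup, and EndPlay destroys the session.
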(event `SetupLobbyMenu`
  (set `self.bShowMouseCursor` true)
  (bind _returnvalue (`|CreateWidget` "/Game/Blueprints/Widgets/WBP_Lobby.WBP_Lobby_C" self))
  (bind _output_get (set `self.LobbyWidget` _returnvalue))
  (`UserWidget.AddToViewport` _output_get 0)
  (`WidgetBlueprintLibrary.SetInputMode_UIOnlyEx` self (`self.LobbyWidget`)))

(event `AssignCharacter`
  (params (CharacterID :type Integer))
  (set `self.SelectedCharacter` CharacterID)
  (`self.CharacterCheck`))

(event `CallUpdate`
  (params (PlayerInfoClass :type "FCharacter Class Reference"))
  ;[1 1 1] Update and Change Possessed Character to New Selection
  (`/Game/Blueprints/Gamemodes/BP_FTDGameMode.SwapCharacter` (cast `/Game/Blueprints/Gamemodes/BP_FTDGameMode` (`GameplayStatics.GetGameMode`) :!pure true) self PlayerInfoClass))

(event `AssignPlayer`
  (params (PlayerClass :type "FCharacter Class Reference"))
  (bind _output_get (set `self.PlayerClass` PlayerClass))
  (`self.CallUpdate` _output_get))

(event `ReadyUp`
  ;[1 1 1] Update Ready/Unready Status
  (if (not (`self.isPlayerReady`))
    (set `self.isPlayerReady` true)
    (bind _asbp_ftdgame_mode (cast `/Game/Blueprints/Gamemodes/BP_FTDGameMode` (`GameplayStatics.GetGameMode`)))
    (`FTDGameMode.PlayerReadyUp` _asbp_ftdgame_mode)))

(event `self.ReceivePossess`
  (params (PossessedPawn :type "Pawn Object Reference"))
  ;[1 1 1] When we Possess an FCharacter Setup the UI
  (bind _asbp_defender (cast `/Game/Blueprints/Character/BP_Defender` PossessedPawn)
    (:`then`
      (`/Game/Blueprints/Character/BP_Defender.SetupUI` _asbp_defender))
    (:`CastFailed`
      (bind _asbp_trapper (cast `/Game/Blueprints/Character/BP_Trapper` PossessedPawn))
      (`/Game/Blueprints/Character/BP_Trapper.SetupUI` _asbp_trapper))))

(event `Unready`
  ;[1 1 1] Update Ready/Unready Status
  (if (`self.isPlayerReady`)
    (set `self.isPlayerReady` false)
    (bind _asbp_ftdgame_mode (cast `/Game/Blueprints/Gamemodes/BP_FTDGameMode` (`GameplayStatics.GetGameMode`)))
    (`FTDGameMode.PlayerUnready` _asbp_ftdgame_mode)))

(event `self.ReceiveEndPlay`
  (params (EndPlayReason :type "EEndPlayReason Enum" :default "Destroyed"))
  (`DestroySessionCallbackProxy.DestroySession` self))

(fn `CharacterCheck`
  (`self.AssignPlayer` (`|GetArrayItem` (`/Game/Blueprints/Gamemodes/BP_FTDGameMode.Characters` (cast `/Game/Blueprints/Gamemodes/BP_FTDGameMode` (`GameplayStatics.GetGameMode`) :!pure true)) (`self.SelectedCharacter`))))

(fn `UserConstructionScript`)